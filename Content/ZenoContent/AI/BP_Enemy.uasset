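; Enemy character that damages the player when a catch succeeds, then halts before resuming movement.
; A box overlap tracks the player in range, and CatchPlayer only acts when its target matches that player.
; A DoOnce gates the catch, setting a material state, applying damage and zeroing walk speed until a delay restores it and resets the gate.
; VisualIndicator maps a color state to the saved base material or an alternate on the mesh.
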(event OnComponentBeginOverlap(Box)
  (params (OverlappedComponent :type Primitive%20Component%20Object%20Reference) (OtherActor :type Actor%20Object%20Reference) (OtherComp :type Primitive%20Component%20Object%20Reference) (OtherBodyIndex :type Integer) (bFromSweep :type Boolean) (SweepResult :type Hit%20Result%20Structure%20%28by%20ref%29))
  (if (== OtherActor (Game|GetPlayerCharacter 0))
    (Variables|Default|SetPlayerInRange OtherActor)))

(event OnComponentEndOverlap(Box)
  (params (OverlappedComponent :type Primitive%20Component%20Object%20Reference) (OtherActor :type Actor%20Object%20Reference) (OtherComp :type Primitive%20Component%20Object%20Reference) (OtherBodyIndex :type Integer))
  (if (== OtherActor (Game|GetPlayerCharacter 0))
    (Variables|Default|SetPlayerInRange 0)))

(event EventCatchPlayer
  (params (TargetActor :type Actor%20Object%20Reference))
  (if (== TargetActor (Variables|Default|GetPlayerInRange))
    (Utilities|FlowControl|DoOnce false :!label _label
      (:Completed
        (Variables|Default|SetMaterialState 2)
        (Game|Damage|ApplyDamage (Variables|Default|GetPlayerInRange) 2e+01 0 self)
        (Variables|/Script/Engine.CharacterMovementComponent|SetMaxWalkSpeed (Variables|Character|GetCharacterMovement) 0.0)
        (Utilities|FlowControl|Delay 5.0)
        (Variables|/Script/Engine.CharacterMovementComponent|SetMaxWalkSpeed (Variables|Character|GetCharacterMovement) 4e+02)
        (goto _label Reset)))))

(event EventBeginPlay
  (Variables|Default|SetBaseMaterial (Rendering|Material|GetMaterial (Variables|Character|GetMesh) 1))
  (Rendering|Material|SetMaterial (Variables|Character|GetMesh) 1 (Variables|Default|GetBaseMaterial)))

(event EventVisualIndicator
  (params (ColorState :type Integer))
  (switch int ColorState
    (:1
      (Rendering|Material|SetMaterial (Variables|Character|GetMesh) 1 (Variables|Default|GetBaseMaterial)))
    (:2
      (Rendering|Material|SetMaterial (Variables|Character|GetMesh) 1 (Utilities|Array|Get(acopy) (Variables|Default|GetMaterial%20Array))))
    (:3
      (Rendering|Material|SetMaterial (Variables|Character|GetMesh) 1 (Utilities|Array|Get(acopy) (Variables|Default|GetMaterial%20Array) 1)))
    (:4
      (Rendering|Material|SetMaterial (Variables|Character|GetMesh) 1 (Utilities|Array|Get(acopy) (Variables|Default|GetMaterial%20Array) 2)))))

(fn ConstructionScript)