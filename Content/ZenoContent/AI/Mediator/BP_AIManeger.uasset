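; BP_AIManeger is a mediator that coordinates which enemy chases the player.
; On BeginPlay it defaults its target to the player character, caches all BP_Enemy actors as seekers and stores the target's max chaser count.
; HandleChaseRequest finds the seeker nearest the player, sends it a catch message and tells the rest to prepare.
; The stored chaser count is not used in that selection, so only one seeker is picked.
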(event EventBeginPlay
  (Variables|Default|GetTargetActor
    (:then
      _)
    (:else
      (Variables|Default|SetTargetActor (Game|GetPlayerCharacter 0))))
  (bind _outactors (Actor|GetAllActorsOfClass "/Game/ZenoContent/AI/BP_Enemy.BP_Enemy_C"))
  (Variables|Default|SetSeekers _outactors)
  (bind _value (Class|BPIHider|MaxChaserCount(Message) (Variables|Default|GetTargetActor)))
  (Variables|Default|SetValue _value))

(fn ConstructionScript)

(fn HandleChaseRequest
  (params (Chaser :type Actor%20Object%20Reference))
  (if (not (== Chaser (Variables|Default|GetTargetActor)))
    (if (Utilities|Array|IsValidIndex (Variables|Default|GetSeekers))
      (Variables|Default|SetClosestDistance 999999.0)
      (Variables|Default|SetActiveChase 0)
      (for (_array_element _array_index) (Variables|Default|GetSeekers)
        (if (< (Math|Vector|VectorLength (- (Transformation|GetActorLocation _array_element) (Transformation|GetActorLocation (Game|GetPlayerCharacter 0)))) (Variables|Default|GetClosestDistance))
          (Variables|Default|SetClosestDistance (Math|Vector|VectorLength (- (Transformation|GetActorLocation _array_element) (Transformation|GetActorLocation (Game|GetPlayerCharacter 0)))))
          (Variables|Default|SetClosestIndex _array_index)))
      (for (_array_element_2 _array_index_2) (Variables|Default|GetSeekers)
        (if (== _array_index_2 (Variables|Default|GetClosestIndex))
          (Class|BPISeeker|CatchPlayer(Message) _array_element_2)
          (else
            (Class|BPISeeker|PreparetoCatch(Message) _array_element_2)))))))