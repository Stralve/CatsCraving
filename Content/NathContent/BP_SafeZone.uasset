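; BP_SafeZone is a zone actor where the player can deposit food they carry.
; A box overlap shows the Interact component when the player pawn enters and hides it when any overlap ends.
; The Store event takes a character reference, decrements its FoodAmount by one if above zero, and prints a success or failure message.
; The deposited food is not recorded in the zone itself.
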(event OnComponentBeginOverlap(Box)
  (params (OverlappedComponent :type Primitive%20Component%20Object%20Reference) (OtherActor :type Actor%20Object%20Reference) (OtherComp :type Primitive%20Component%20Object%20Reference) (OtherBodyIndex :type Integer) (bFromSweep :type Boolean) (SweepResult :type Hit%20Result%20Structure%20%28by%20ref%29))
  ;[0.05098 0.05098 0.05098] Widget interaction visibility
  (if (== OtherActor (Game|Player|GetPlayerPawn 0))
    (Rendering|SetVisibility (Variables|Default|GetInteract) true false)))

(event OnComponentEndOverlap(Box)
  (params (OverlappedComponent :type Primitive%20Component%20Object%20Reference) (OtherActor :type Actor%20Object%20Reference) (OtherComp :type Primitive%20Component%20Object%20Reference) (OtherBodyIndex :type Integer))
  ;[0.05098 0.05098 0.05098] Widget interaction visibility
  (Rendering|SetVisibility (Variables|Default|GetInteract) false false))

(event EventStore
  (params (CharRef :type BP%20Third%20Person%20Character%20Object%20Reference))
  ;[0.05098 0.05098 0.05098] Storing food
  (bind _output_get (Variables|Default|SetChar%20Ref CharRef))
  (if (> (Variables|/Game/ThirdPerson/Blueprints/BP_ThirdPersonCharacter.BP_ThirdPersonCharacter_C|GetFoodAmount _output_get) 0)
    (Development|PrintString "Food has been deposited :D")
    (bind _result (Math|Integer|DecrementInt (Variables|/Game/ThirdPerson/Blueprints/BP_ThirdPersonCharacter.BP_ThirdPersonCharacter_C|GetFoodAmount (Variables|Default|GetChar%20Ref)))
      (:%20%20
        (Variables|/Game/ThirdPerson/Blueprints/BP_ThirdPersonCharacter.BP_ThirdPersonCharacter_C|SetFoodAmount (Variables|Default|GetChar%20Ref) _result)))
    (else
      (Development|PrintString "You have no food :("))))

(fn ConstructionScript)