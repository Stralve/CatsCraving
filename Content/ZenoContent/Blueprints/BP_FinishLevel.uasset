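; Level-finish trigger actor that marks where the player delivers a required amount or type of food.
; The construction script builds a "Deliver … Food" text label from the FoodValidation value.
; A collision box detects actors tagged "Character" entering or leaving and sends InRangeMessage to the game mode with the in-range state and FoodValidation, leaving the delivery logic to that game mode.
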(event OnComponentBeginOverlap(Box_Collision)
  (params (OverlappedComponent :type Primitive%20Component%20Object%20Reference) (OtherActor :type Actor%20Object%20Reference) (OtherComp :type Primitive%20Component%20Object%20Reference) (OtherBodyIndex :type Integer) (bFromSweep :type Boolean) (SweepResult :type Hit%20Result%20Structure%20%28by%20ref%29))
  (if (Actor|ActorHasTag OtherActor "Character")
    (Class|BPIFoodValidation|InRange(Message) (Game|GetGameMode) true (Variables|Default|GetFoodValidation))))

(event OnComponentEndOverlap(Box_Collision)
  (params (OverlappedComponent :type Primitive%20Component%20Object%20Reference) (OtherActor :type Actor%20Object%20Reference) (OtherComp :type Primitive%20Component%20Object%20Reference) (OtherBodyIndex :type Integer))
  (if (Actor|ActorHasTag OtherActor "Character")
    (Class|BPIFoodValidation|InRange(Message) (Game|GetGameMode) false (Variables|Default|GetFoodValidation))))

(event EventBeginPlay)

(event Collision|EventActorBeginOverlap
  (params (OtherActor :type Actor%20Object%20Reference)))

(event EventTick
  (params (DeltaSeconds :type Float%20%28single-precision%29)))

(fn ConstructionScript
  (Rendering|Components|TextRender|SetText (Variables|Default|GetTextRender) (Utilities|Text|ToText(String) (Utilities|String|Append "Deliver" " " (Utilities|String|ToString(Integer) (Variables|Default|GetFoodValidation)) " " "Food"))))